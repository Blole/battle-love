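; Player controller that lets one player steer a character made of two physics-linked halves.
; On BeginPlay it spawns two PlayerHalf actors offset along X and joins their spheres with the left half's physics constraint.
; Separate X and Y input axes drive each half's movement functions, with only the left half's Y axis inverted.
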(event `self.ReceiveBeginPlay`
  (bind _returnvalue (`KismetMathLibrary.MakeTransform` (0.0 0.0 100.0)))
  (bind _lefthalf (`self.LeftHalf`))
  (bind _returnvalue_2 (`|SpawnActorFromClass` "/Game/Blueprints/PlayerHalf.PlayerHalf_C" _returnvalue))
  (set `self.LeftHalf` _returnvalue_2)
  (bind _returnvalue_3 (`|SpawnActorFromClass` "/Game/Blueprints/PlayerHalf.PlayerHalf_C" (`KismetMathLibrary.ComposeTransforms` _returnvalue (`KismetMathLibrary.MakeTransform` (100.0 0.0 0.0)))))
  (set `self.RightHalf` _returnvalue_3)
  (`PhysicsConstraintComponent.SetConstrainedComponents` (`/Game/Blueprints/PlayerHalf.PhysicsConstraint1` _lefthalf) (`/Game/Blueprints/PlayerHalf.Sphere1` _lefthalf) "None" (`/Game/Blueprints/PlayerHalf.Sphere1` (`self.RightHalf`)) "None"))

(event `InputAxis|LeftHalfX`
  (params (AxisValue :type "Float (single-precision)"))
  (`/Game/Blueprints/PlayerHalf.MoveX` (`self.LeftHalf`) AxisValue))

(event `InputAxis|LeftHalfY`
  (params (AxisValue :type "Float (single-precision)"))
  (`/Game/Blueprints/PlayerHalf.Move Y` (`self.LeftHalf`) (* AxisValue -1.0)))

(event `InputAxis|RightHalfX`
  (params (AxisValue :type "Float (single-precision)"))
  (`/Game/Blueprints/PlayerHalf.MoveX` (`self.RightHalf`) AxisValue))

(event `InputAxis|RightHalfY`
  (params (AxisValue :type "Float (single-precision)"))
  (`/Game/Blueprints/PlayerHalf.Move Y` (`self.RightHalf`) AxisValue))

(fn `UserConstructionScript`)