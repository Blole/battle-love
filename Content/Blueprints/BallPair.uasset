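; BallPair is a Blueprint that drives a left and a right ball through physics impulses.
; MoveLeft and MoveRight each scale a direction by MoveForce and call AddImpulse, with velocity change off so mass affects the result.
; Per-side X and Y wrappers turn a scalar amount into an axis vector and pass it to these functions.
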(fn `Move Left`
  (params (Direction :type "Object.Vector Structure"))
  (`PrimitiveComponent.AddImpulse` (* Direction (`self.MoveForce`))))

(fn `Move Left Y`
  (params (Amount :type "Float (double-precision)"))
  (`self.Move Left` (* (0.0 1.0 0.0) Amount)))

(fn `Move Right`
  (params (Direction :type "Object.Vector Structure"))
  (`PrimitiveComponent.AddImpulse` (* Direction (`self.MoveForce`))))

(fn `Move Right X`
  (params (Amount :type "Float (double-precision)"))
  (`self.Move Right` (* (1.0 0.0 0.0) Amount)))

(fn `Move Right Y`
  (params (Amount :type "Float (double-precision)"))
  (`self.Move Right` (* (0.0 1.0 0.0) Amount)))

(fn `MoveLeftX`
  (params (Amount :type "Float (double-precision)"))
  (`self.Move Left` (* (1.0 0.0 0.0) Amount)))

(fn `UserConstructionScript`)